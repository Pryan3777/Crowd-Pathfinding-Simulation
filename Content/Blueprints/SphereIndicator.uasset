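; SphereIndicator is a component that gives its owning actor a colored, flattened sphere marker, offset below the actor's origin.
; On BeginPlay it adds the hidden mesh to the owner and creates a dynamic material, whose Color parameter is rewritten every Tick from the value set by UpdateColor.
; SetVisibility shows or hides the marker until Cancel hides it and blocks it from being shown again.
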(event `self.ReceiveBeginPlay`
  (bind _returnvalue (`|AddComponentByClass` (`self.GetOwner`) "/Script/Engine.StaticMeshComponent" false (`KismetMathLibrary.MakeTransform` (0.0 0.0 -95.0) (struct) (1.0 1.0 0.1))))
  (bind _output_get (set `self.Mesh` _returnvalue))
  (`SceneComponent.SetVisibility` _output_get false true)
  (`StaticMeshComponent.SetStaticMesh` _output_get "/Game/StarterContent/Shapes/Shape_Sphere.Shape_Sphere")
  (bind _returnvalue_2 (`PrimitiveComponent.CreateDynamicMaterialInstance` _output_get 0 null "None"))
  (set `self.Material` _returnvalue_2))

(event `self.ReceiveTick`
  (params (DeltaSeconds :type "Float (single-precision)"))
  (`MaterialInstanceDynamic.SetVectorParameterValue` (`self.Material`) "Color" (`self.Color`)))

(fn `Cancel`
  (set `self.Cancelled` true)
  (`SceneComponent.SetVisibility` (`self.Mesh`) false true))

(fn `SetVisibility`
  (params (Show :type Boolean))
  (`SceneComponent.SetVisibility` (`self.Mesh`) (and Show (not (`self.Cancelled`))) true))

(fn `UpdateColor`
  (params (NewColor :type "LinearColor Structure"))
  (set `self.Color` NewColor))