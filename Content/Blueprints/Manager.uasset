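; Scene manager that gives the player and civilians uniquely colored sphere indicators from a shuffled palette, assigned until colors run out.
; Tick polls three toggles through paired DoOnce nodes, intended to act only on changes.
; These drive debug drawing on civilians and nav nodes, blending between third-person and overhead cameras, and indicator visibility.
; Cancel cancels civilian indicators one per call, tracked by a running count.
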(event `self.ReceiveBeginPlay`
  (bind _colors (`self.Colors`))
  (bind _colors_2 (`self.Colors`))
  (`KismetArrayLibrary.Array_Shuffle` _colors)
  (bind _returnvalue (`GameplayStatics.GetActorOfClass` "/Game/ThirdPerson/Blueprints/BP_ThirdPersonCharacter.BP_ThirdPersonCharacter_C"))
  (bind _returnvalue_2 (`|AddComponentByClass` _returnvalue "/Game/Blueprints/SphereIndicator.SphereIndicator_C"))
  (`/Game/Blueprints/SphereIndicator.UpdateColor` _returnvalue_2 (`|GetArrayItem` _colors))
  (`KismetArrayLibrary.Array_Remove` _colors)
  (bind _outactors (`GameplayStatics.GetAllActorsOfClass` "/Script/PPP.Civilian"))
  (bind _output_get (set `self.Civilians` _outactors))
  (for _array_element _output_get
    (if (== (`KismetArrayLibrary.Array_Length` (`self.Colors`)) 0)
      (break)
      (else
        (bind _returnvalue_3 (`|AddComponentByClass` _array_element "/Game/Blueprints/SphereIndicator.SphereIndicator_C"))
        (`/Game/Blueprints/SphereIndicator.UpdateColor` _returnvalue_3 (`|GetArrayItem` _colors_2))
        (`KismetArrayLibrary.Array_Remove` _colors_2)))))

(event `self.ReceiveTick`
  (params (DeltaSeconds :type "Float (single-precision)"))
  (bind _draw (`self.Draw`))
  (bind _thirdpersoncamera (`self.ThirdPersonCamera`))
  (`|ExecutionSequence`
    (:`then_0`
      (if (`self.Draw`)
        (`/Engine/EditorBlueprintResources/StandardMacros.DoOnce` false :!label _label
          (:`Completed`
            (`|ExecutionSequence`
              (:`then_0`
                (goto _label_2 :!via `Reset`))
              (:`then_1`
                _))))
        (else
          (`/Engine/EditorBlueprintResources/StandardMacros.DoOnce` false :!label _label_2
            (:`Completed`
              (`|ExecutionSequence`
                (:`then_0`
                  (goto _label :!via `Reset`))
                (:`then_1`
                  _))))))
      (bind _outactors (`GameplayStatics.GetAllActorsOfClass` "/Script/PPP.Civilian"))
      (for _array_element _outactors
        (set `Civilian.draw` (`self.Draw`) _array_element))
      (bind _outactors_2 (`GameplayStatics.GetAllActorsOfClass` "/Script/PPP.NavNode"))
      (for _array_element_2 _outactors_2
        (`self.SetActorHiddenInGame` _array_element_2 (not _draw))
        (set `NavNode.draw` _draw _array_element_2)))
    (:`then_1`
      (if _thirdpersoncamera
        (`/Engine/EditorBlueprintResources/StandardMacros.DoOnce` false :!label _label_3
          (:`Completed`
            (`|ExecutionSequence`
              (:`then_0`
                (goto _label_4 :!via `Reset`))
              (:`then_1`
                _))))
        (else
          (`/Engine/EditorBlueprintResources/StandardMacros.DoOnce` false :!label _label_4
            (:`Completed`
              (`|ExecutionSequence`
                (:`then_0`
                  (goto _label_3 :!via `Reset`))
                (:`then_1`
                  _))))))
      (bind _returnvalue (`InputDeviceLibrary.GetPlayerControllerFromInputDevice` (`InputDeviceLibrary.GetDefaultInputDevice`)))
      (bind _returnvalue_2 (`GameplayStatics.GetActorOfClass` "/Game/ThirdPerson/Blueprints/BP_ThirdPersonCharacter.BP_ThirdPersonCharacter_C"))
      (`PlayerController.SetViewTargetWithBlend` _returnvalue (select `bool` _thirdpersoncamera :`false` (`self.CameraOverhead`) :`true` _returnvalue_2 :!type "Actor Object Reference") 0.0 "VTBlend_Linear" 0.0 false))
    (:`then_2`
      (if (`self.ShowColors`)
        (`/Engine/EditorBlueprintResources/StandardMacros.DoOnce` false :!label _label_5
          (:`Completed`
            (`|ExecutionSequence`
              (:`then_0`
                (goto _label_6 :!via `Reset`))
              (:`then_1`
                _))))
        (else
          (`/Engine/EditorBlueprintResources/StandardMacros.DoOnce` false :!label _label_6
            (:`Completed`
              (`|ExecutionSequence`
                (:`then_0`
                  (goto _label_5 :!via `Reset`))
                (:`then_1`
                  _))))))
      (bind _returnvalue_3 (`GameplayStatics.GetActorOfClass` "/Game/ThirdPerson/Blueprints/BP_ThirdPersonCharacter.BP_ThirdPersonCharacter_C"))
      (`/Game/Blueprints/SphereIndicator.SetVisibility` (`self.GetComponentByClass` _returnvalue_3 "/Game/Blueprints/SphereIndicator.SphereIndicator_C") (`self.ShowColors`))
      (for _array_element_3 (`self.Civilians`)
        (bind _returnvalue_4 (`self.GetComponentByClass` _array_element_3 "/Game/Blueprints/SphereIndicator.SphereIndicator_C"))
        (`/Engine/EditorBlueprintResources/StandardMacros.IsValid` _returnvalue_4
          (:`Is Valid`
            (`/Game/Blueprints/SphereIndicator.SetVisibility` _returnvalue_4 (`self.ShowColors`))))))))

(fn `Cancel`
  (bind _civilians (`self.Civilians`))
  (bind _cancelledcount (`self.CancelledCount`))
  (bind _returnvalue (`self.GetComponentByClass` (`|GetArrayItem` _civilians _cancelledcount) "/Game/Blueprints/SphereIndicator.SphereIndicator_C"))
  (if (< _cancelledcount (`KismetArrayLibrary.Array_Length` _civilians))
    (`/Engine/EditorBlueprintResources/StandardMacros.IsValid` _returnvalue
      (:`Is Valid`
        (`/Game/Blueprints/SphereIndicator.Cancel` _returnvalue)
        (set `self.CancelledCount` (+ (`self.CancelledCount`) 1))))))

(fn `UserConstructionScript`)